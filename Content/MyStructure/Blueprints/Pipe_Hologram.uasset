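; Hologram slot for a placeable pipe that opens the door linked to it by ID.
; When a BP_Placeable_Pipe overlaps it and a BP_Door's DoorID matches PlateID, it destroys the pipe, applies the wall pipe material to ObjectIndicator and opens that door.
; When a pipe's overlap ends, it waits a few seconds, searches all doors for the match again and closes it.
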(event `self.ReceiveActorBeginOverlap`
  (params (OtherActor :type "Actor Object Reference"))
  (bind _bp_door (`self.BP_Door`))
  ;[1 0.8393 0] Open Door Activation
  (bind _asbp_placeable_pipe (cast `/Game/MyStructure/Blueprints/BP_Placeable_Pipe` OtherActor))
  (bind _outactors (`GameplayStatics.GetAllActorsOfClass` "/Game/MyStructure/Blueprints/BP_Door.BP_Door_C"))
  (for _array_element _outactors
    (if (== (`/Game/MyStructure/Blueprints/BP_Door.DoorID` _array_element) (`self.Plate_ID`))
      (set `self.BP_Door` _array_element)
      (`self.K2_DestroyActor` _asbp_placeable_pipe)
      (`PrimitiveComponent.SetMaterial` (`self.ObjectIndicator`) 0 "/Game/MyStructure/Materials/Tx_WallPipe.Tx_WallPipe")))
  (`/Engine/EditorBlueprintResources/StandardMacros.IsValid` _bp_door
    (:`Is Valid`
      (`/Game/MyStructure/Blueprints/BP_Door.Open` _bp_door))))

(event `self.ReceiveActorEndOverlap`
  (params (OtherActor :type "Actor Object Reference"))
  (bind _bp_door (`self.BP_Door`))
  ;[1 0.7818 0] Close Door Activation
  (cast `/Game/MyStructure/Blueprints/BP_Placeable_Pipe` OtherActor)
  (`KismetSystemLibrary.Delay` 3.0)
  (bind _outactors (`GameplayStatics.GetAllActorsOfClass` "/Game/MyStructure/Blueprints/BP_Door.BP_Door_C"))
  (for _array_element _outactors
    (if (== (`/Game/MyStructure/Blueprints/BP_Door.DoorID` _array_element) (`self.Plate_ID`))
      (set `self.BP_Door` _array_element)))
  (`/Engine/EditorBlueprintResources/StandardMacros.IsValid` _bp_door
    (:`Is Valid`
      (`/Game/MyStructure/Blueprints/BP_Door.Close` _bp_door))))

(fn `UserConstructionScript`)